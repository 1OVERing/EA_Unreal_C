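; Test AI controller for monsters that starts their behavior tree and relays perception events.
; On BeginPlay it runs BT_MonsterMaster_Test, then seeds the blackboard with the controller's own location as patrol origin and a fixed patrol radius.
; AI perception target updates are forwarded to BP_Monster's PerceptionUpdate, reached by casting the controller's owner rather than the controlled pawn.
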(event OnTargetPerceptionUpdated(AIPerception)
  (params (Actor :type Actor%20Object%20Reference) (Stimulus :type AI%20Stimulus%20Structure))
  (bind _asbp_monster (Utilities|Casting|CastToBP_Monster (Components|GetOwner)))
  (Default|PerceptionUpdate _asbp_monster Actor Stimulus))

(event EventBeginPlay
  (AI|RunBehaviorTree "/Game/Blueprints/Monster/BT_MonsterMaster_Test.BT_MonsterMaster_Test")
  (AI|Components|Blackboard|SetValueasVector (Variables|Default|GetBlackboard) (Utilities|Name|MakeLiteralName "OriginLocation") (Transformation|GetActorLocation))
  (AI|Components|Blackboard|SetValueasFloat (Variables|Default|GetBlackboard) (Utilities|Name|MakeLiteralName "PatrolRadius") (Math|Float|MakeLiteralFloat 1e+03)))

(fn ConstructionScript)