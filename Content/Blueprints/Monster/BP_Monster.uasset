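; Katana-wielding AI monster character that locks onto the player once perceived, storing it in the blackboard and entering combat mode.
; Custom movement follows synchronous navmesh waypoints by feeding movement scale and sprint to the anim instance, with stuck detection and turn-in-place montages.
; In combat it faces the target while moving directionally.
; Damage plays directional hit montages; helpers swap weapon sockets and time catch-attack montages.
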(event OnTargetPerceptionUpdated(AIPerception)
  (params (Actor :type Actor%20Object%20Reference) (Stimulus :type AI%20Stimulus%20Structure))
  (CallFunction|PerceptionUpdate Actor Stimulus))

(event EventTick
  (params (DeltaSeconds :type Float%20%28single-precision%29)))

(event Game|Damage|EventAnyDamage
  (params (Damage :type Float%20%28single-precision%29) (DamageType :type Damage%20Type%20Object%20Reference) (InstigatedBy :type Controller%20Object%20Reference) (DamageCauser :type Actor%20Object%20Reference))
  (if (!= DamageCauser 0)
    (CallFunction|PlayHitAnimMontage DamageCauser)))

(fn ConstructionScript
  (Variables|Default|SetAIControllerClass "/Game/Blueprints/Monster/IC_MonsterMasterController_Test.IC_MonsterMasterController_Test_C"))

(fn PlayHitAnimMontage
  (params (Causer :type Actor%20Object%20Reference))
  (bind _returnvalue (Transformation|GetActorLocation Causer))
  (bind (_rightsacle _forwardscale) (CallFunction|FindVectortoDirection _returnvalue))
  (Animation|StopAnimMontage 0)
  (Utilities|FlowControl|Sequence
    (:then_0)
    (:then_1
      (if (> _forwardscale 0.5)
        (LocalVariables|SetNormalHitNum 0)
        (elif (< _forwardscale -0.5)
          (LocalVariables|SetNormalHitNum 1)
          (elif (> _rightsacle 0.5)
            (LocalVariables|SetNormalHitNum 2)
            (elif (< _rightsacle -0.5)
              (LocalVariables|SetNormalHitNum 3))))))
    (:then_2
      (Animation|PlayAnimMontage (Utilities|Select :Index (LocalVariables|GetNormalHitNum) :Option%200 "/Game/Animations/EnemyKatana/Montage/AM_KatanaHit_Back.AM_KatanaHit_Back" :Option%201 "/Game/Animations/EnemyKatana/Montage/AM_KatanaHit_Forward.AM_KatanaHit_Forward" :Option%202 "/Game/Animations/EnemyKatana/Montage/AM_KatanaHit_Left.AM_KatanaHit_Left" :Option%203 "/Game/Animations/EnemyKatana/Montage/AM_KatanaHit_Right.AM_KatanaHit_Right") 1.0 "None"))))

(fn FindVectortoDirection
  (params (Location :type Vector))
  (bind (_x _y) (Math|Vector|BreakVector Location))
  (bind _returnvalue (Transformation|GetActorLocation))
  (bind _returnvalue_2 (- (Math|Vector|MakeVector _x _y 0.0) (Math|Vector|MakeVector (.x _returnvalue) (.y _returnvalue) 0.0)))
  (bind _returnvalue_3 (Math|Vector|Normalize _returnvalue_2))
  (return (Math|Float|Lerp 1.0 -1.0 (/ (Math|Trig|RadiansToDegrees (Math|Trig|Acos(Degrees) (Math|Vector|DotProduct _returnvalue_3 (Transformation|GetActorRightVector)))) 1.8e+02)) (Math|Float|Lerp 1.0 -1.0 (/ (Math|Trig|RadiansToDegrees (Math|Trig|Acos(Degrees) (Math|Vector|DotProduct _returnvalue_3 (Transformation|GetActorForwardVector)))) 1.8e+02))))

(fn WeaponEquip
  (params (Equip :type Boolean))
  (if Equip
    (LocalVariables|SetSocketName "ik_hand_gun")
    (CallFunction|SetCombatMode true)
    (else
      (LocalVariables|SetSocketName "KatanaSheath")
      (CallFunction|SetCombatMode false)))
  (Transformation|AttachComponentToComponent (Variables|Default|GetSK_Weapon) (Variables|Character|GetMesh) (LocalVariables|GetSocketName) "SnapToTarget" "SnapToTarget" "SnapToTarget" true))

(fn GetNextMovePoint
  (bind _waypoints (Variables|Default|GetWayPoints))
  (if (not (Utilities|Array|IsEmpty (Variables|Default|GetWayPoints)))
    (if (> (Math|Vector|Distance(Vector) (Transformation|GetActorLocation) (Utilities|Array|Get(acopy) (Variables|Default|GetWayPoints))) 1e+02) :!label _label
      (return true (Utilities|Array|Get(acopy) (Variables|Default|GetWayPoints)))
      (else
        (Utilities|Array|RemoveIndex _waypoints)
        (if (<= (Utilities|Array|Length _waypoints) 0)
          (return false "0, 0, 0")
          (else
            (goto _label)))))))

(fn FindWayPoint
  (params (InputPin :type Vector))
  (bind _returnvalue (Class|NavigationSystemV1|FindPathtoLocationSynchronously (Class|NavigationSystemV1|GetNavigationSystem) (Transformation|GetActorLocation) InputPin 0 0))
  (if (> (Utilities|Array|Length (Variables|/Script/NavigationSystem.NavigationPath|GetPathPoints _returnvalue)) 0)
    (Variables|Default|SetWayPoints (Variables|/Script/NavigationSystem.NavigationPath|GetPathPoints _returnvalue))
    (bind _validwaypoint (CallFunction|GetNextMovePoint))
    (return _validwaypoint)
    (else
      (return false))))

(fn MoveCheck
  (if (CallFunction|InRotation)
    (return true)
    (elif (Utilities|Operators|NotEqual(!=) (Variables|Default|GetPrevLocation) (Transformation|GetActorLocation) 0.0)
      (Variables|Default|SetPrevLocation (Transformation|GetActorLocation))
      (Variables|Default|SetStopLocationTime 0.0)
      (return true)
      (else
        (bind _output_get (Variables|Default|SetStopLocationTime (+ (Variables|Default|GetStopLocationTime) (Utilities|Time|GetWorldDeltaSeconds))))
        (if (> _output_get 1.0)
          (return false)
          (else
            (return true)))))))

(fn RotationCheck
  (params (Target :type Vector%20%28by%20ref%29))
  (if (and (CallFunction|IsCombatMode) (> (Math|Float|Absolute(Float) (CallFunction|FindAngle Target)) 8e+01))
    (CallFunction|PlayRotation Target (CallFunction|FindAngle Target))
    (return true)
    (else
      (bind _returnvalue (Transformation|SetActorRotation (Math|Rotator|MakeRotator 0.0 0.0 (.yaw (Math|Rotator|FindLookatRotation (Transformation|GetActorLocation) Target)))))
      (return _returnvalue))))

(fn PlayRotation
  (params (TargetLocation :type Vector) (Angle :type Float%20%28double-precision%29))
  (if (>= Angle 0.0)
    (if (> (Math|Float|Absolute(Float) Angle) 1.7e+02)
      (Animation|PlayAnimMontage "/Game/Animations/EnemyKatana/Montage/AM_KatanaTurnR180.AM_KatanaTurnR180" 1.0 "None")
      (else
        (Animation|PlayAnimMontage "/Game/Animations/EnemyKatana/Montage/AM_KatanaTurnR90.AM_KatanaTurnR90" 1.0 "None")))
    (elif (> (Math|Float|Absolute(Float) Angle) 1.7e+02)
      (Animation|PlayAnimMontage "/Game/Animations/EnemyKatana/Montage/AM_KatanaTurnL180.AM_KatanaTurnL180" 1.0 "None")
      (else
        (Animation|PlayAnimMontage "/Game/Animations/EnemyKatana/Montage/AM_KatanaTurnL90.AM_KatanaTurnL90" 1.0 "None")))))

(fn FindAngle
  (params (TargetLocation :type Vector))
  (bind _returnvalue (Transformation|GetActorLocation))
  (bind _returnvalue_2 (Transformation|GetActorForwardVector))
  (bind _returnvalue_3 (Math|Rotator|FindLookatRotation _returnvalue TargetLocation))
  (bind (_x _y) (Math|Vector|BreakVector _returnvalue_2))
  (bind _returnvalue_4 (Math|Vector|GetForwardVector _returnvalue_3))
  (bind (_x_2 _y_2) (Math|Vector|BreakVector _returnvalue_4))
  (return (- (Class|KismetMathLibrary|DegAtan2 _x _y) (Class|KismetMathLibrary|DegAtan2 _x_2 _y_2))))

(fn InRotation
  (bind _returnvalue (Animation|GetCurrentMontage :!class /Script/Engine.Character))
  (return (Math|Boolean|ORBoolean (== _returnvalue "/Game/Animations/EnemyKatana/Montage/AM_KatanaTurnL90.AM_KatanaTurnL90") (== _returnvalue "/Game/Animations/EnemyKatana/Montage/AM_KatanaTurnL180.AM_KatanaTurnL180") (== _returnvalue "/Game/Animations/EnemyKatana/Montage/AM_KatanaTurnR90.AM_KatanaTurnR90") (== _returnvalue "/Game/Animations/EnemyKatana/Montage/AM_KatanaTurnR180.AM_KatanaTurnR180"))))

(fn IsCombatMode
  (bind _asea_master_anim_instance (Utilities|Casting|CastToEA_MasterAnimInstance (Components|SkeletalMesh|GetAnimInstance (Variables|Character|GetMesh))))
  (return (Variables|/Script/EA_Unreal_C.EA_MasterAnimInstance|GetCombatMode _asea_master_anim_instance)))

(fn PerceptionUpdate
  (params (TargetActor :type Actor%20Object%20Reference) (CurrentStimulus :type AI%20Stimulus%20Structure))
  (if (and (== TargetActor (Game|Player|GetPlayerPawn 0)) (.bSuccessfullySensed (Utilities|Struct|BreakAIStimulus CurrentStimulus)))
    (CallFunction|SetTargetActor TargetActor)
    (CallFunction|SetHitParams TargetActor)))

(fn SetTargetActor
  (params (TargetActor :type Actor%20Object%20Reference))
  (AI|Components|Blackboard|SetValueasObject (Variables|/Script/AIModule.AIController|GetBlackboard (AI|GetAIController self)) (Utilities|Name|MakeLiteralName "TargetActor") TargetActor))

(fn SetHitParams
  (params (TargetActor :type Actor%20Object%20Reference))
  (CallFunction|SetCombatMode true)
  (CallFunction|SetTargetActor TargetActor))

(fn SetCombatMode
  (params (CombatMode :type Boolean))
  (bind _asea_master_anim_instance (Utilities|Casting|CastToEA_MasterAnimInstance (Components|SkeletalMesh|GetAnimInstance (Variables|Character|GetMesh))))
  (Class|EAMasterAnimInstance|SetCombatMode _asea_master_anim_instance CombatMode))

(fn SetHitTimer
  (params (HitTime :type Float%20%28double-precision%29))
  (Utilities|Time|ClearandInvalidateTimerbyHandle (Variables|Default|GetHitTimer))
  (bind _returnvalue (Utilities|Time|SetTimerbyFunctionName 0 "EndHitTimer" HitTime))
  (Variables|Default|SetHitTimer _returnvalue)
  (CallFunction|SetHitParams))

(fn EndHitTimer
  (Utilities|Time|ClearandInvalidateTimerbyHandle (Variables|Default|GetHitTimer)))

(fn IsHitReaction
  (return (Utilities|Time|IsTimerActivebyHandle (Variables|Default|GetHitTimer))))

(fn CombatMove
  (params (TargetLocation :type Vector))
  (bind _waypoints (Variables|Default|GetWayPoints))
  (bind _output (Utilities|Array|Get(acopy) _waypoints))
  (bind (_rightsacle _forwardscale) (CallFunction|FindVectortoDirection _output))
  (bind _targetactor (CallFunction|GetTargetActor))
  (if (and (not (CallFunction|InRotation)) (< (Math|Float|Absolute(Float) (CallFunction|FindAngle (Transformation|GetActorLocation _targetactor))) 8e+01))
    (bind _returnvalue (Transformation|SetActorRotation (Math|Rotator|FindLookatRotation (Transformation|GetActorLocation) (Transformation|GetActorLocation _targetactor))))
    (if _returnvalue
      (CallFunction|SetMovementScale (Math|Vector2D|MakeVector2D _rightsacle _forwardscale) :!label _label)
      (bind _targetactor_2 (CallFunction|GetTargetActor))
      (if (> (Math|Vector|Distance(Vector) (Transformation|GetActorLocation _targetactor_2) (Transformation|GetActorLocation)) 3e+02)
        (CallFunction|SetSprint true))
      (return (< (Math|Vector|Distance(Vector) (Transformation|GetActorLocation _targetactor_2) (Transformation|GetActorLocation)) 1e+01)))
    (else
      (CallFunction|PlayRotation (Transformation|GetActorLocation _targetactor) (CallFunction|FindAngle (Transformation|GetActorLocation _targetactor)))
      (goto _label))))

(fn GetTargetActor
  (bind _as액터 (Utilities|Casting|CastToActor (AI|Components|Blackboard|GetValueasObject (AI|GetBlackboard (AI|GetAIController self)) (Utilities|Name|MakeLiteralName "TargetActor"))))
  (return _as액터))

(fn SetMovementScale
  (params (Scale :type Vector%202D%20Structure))
  (bind _asea_master_anim_instance (Utilities|Casting|CastToEA_MasterAnimInstance (Components|SkeletalMesh|GetAnimInstance (Variables|Character|GetMesh))))
  (Class|EAMasterAnimInstance|SetMovementScale _asea_master_anim_instance Scale))

(fn SetSprint
  (params (Sprint :type Boolean))
  (bind _asea_master_anim_instance (Utilities|Casting|CastToEA_MasterAnimInstance (Components|SkeletalMesh|GetAnimInstance (Variables|Character|GetMesh))))
  (Class|EAMasterAnimInstance|SetSprint _asea_master_anim_instance Sprint))

(fn CustomMoveEnd
  (bind _asea_master_anim_instance (Utilities|Casting|CastToEA_MasterAnimInstance (Components|SkeletalMesh|GetAnimInstance (Variables|Character|GetMesh))))
  (Class|EAMasterAnimInstance|SetMovementScale _asea_master_anim_instance (Math|Vector2D|MakeVector2D 0.0 0.0))
  (Utilities|Array|Clear (Variables|Default|GetWayPoints))
  (Variables|Default|SetStopLocationTime 0.0)
  (CallFunction|SetSprint false)
  (Development|PrintString "EndMove")
  (return true))

(fn CustomMoveto
  (params (MoveToLocation :type Vector :default "0, 0, 0"))
  (Utilities|FlowControl|Sequence
    (:then_0
      (if (Utilities|Array|IsEmpty (Variables|Default|GetWayPoints))
        (bind _validwaypoint (CallFunction|FindWayPoint MoveToLocation))
        (if _validwaypoint
          (if (CallFunction|IsHitReaction)
            (return true))
          (else
            (return true)))))
    (:then_1
      (bind _valid (CallFunction|MoveCheck))
      (if (not _valid)
        (return true)))
    (:then_2
      (bind (_validwaypoint_2 _nextmovepoint) (CallFunction|GetNextMovePoint))
      (if _validwaypoint_2
        (if (CallFunction|IsCombatMode)
          (bind _finish (CallFunction|CombatMove _nextmovepoint))
          (return _finish)
          (else
            (if (CallFunction|InRotation)
              _
              (else
                (bind _returnvalue (CallFunction|RotationCheck _nextmovepoint))
                (if _returnvalue
                  _
                  (else
                    (return true)))))
            (bind _asea_master_anim_instance (Utilities|Casting|CastToEA_MasterAnimInstance (Components|SkeletalMesh|GetAnimInstance (Variables|Character|GetMesh))))
            (Class|EAMasterAnimInstance|SetMovementScale _asea_master_anim_instance (Math|Vector2D|MakeVector2D 0.0 1.0))
            (return false)))
        (else
          (return true))))))

(fn PlayCatchAttack
  (params (montage :type Anim%20Montage%20Object%20Reference) (sectionName :type Name :default "None"))
  (bind _returnvalue (Animation|PlayAnimMontage self montage 1.0 sectionName))
  (CallFunction|SetHitTimer _returnvalue)
  (return true))