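; AC_WorldMapIconComponent is an actor component that reports its owner's position as a map icon to the player's HUD.
; Each Tick compares the owner's location with the cached previous one, so updates go out only after movement.
; When the location changes and the icon image is valid, it sends UpdateIconMessage to player 0's HUD with owner, display name, image, size and 2D location.
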(event EventBeginPlay)

(event EventTick
  (params (DeltaSeconds :type Float%20%28single-precision%29))
  (bind _returnvalue (Components|GetOwner))
  (if (Utilities|Operators|NotEqual(!=) (Variables|Default|GetPrevLocation) (Transformation|GetActorLocation (Components|GetOwner)) 0.0)
    (Variables|Default|SetPrevLocation (Transformation|GetActorLocation (Components|GetOwner)))
    (bind _iconimage (Variables|Icon|GetIconImage)
      (:then
        (Class|BPIWorldMap|UpdateIcon(Message) (HUD|GetHUD (Game|GetPlayerController 0)) _returnvalue (Utilities|Struct|MakeF_IconData (Utilities|GetDisplayName _returnvalue) _iconimage (Variables|Icon|GetIconSize) (Math|Conversions|ToVector2D(Vector) (Transformation|GetActorLocation _returnvalue)) false)))
      (:else))))