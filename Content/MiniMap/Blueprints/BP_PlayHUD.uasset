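; HUD that creates the minimap widget and manages the icons shown on it.
; Create, update and remove events edit icon data keyed by owner display name, then redraw the map texture and all icons into a render target.
; Icon positions derive from world location and the MapSize material parameter collection value, with axes swapped.
; Tick writes player location to that collection, and new icons flagged ScreenLook also get widget indicators.
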(event EventBeginPlay
  (bind _returnvalue (UserInterface|CreateWidget "/Game/MiniMap/UI/UMG_Minimap.UMG_Minimap_C"))
  (UserInterface|Viewport|AddtoViewport _returnvalue 0)
  (Variables|Default|SetUMG_Minimap _returnvalue)
  (CallFunction|DrawMap)
  (CallFunction|DrawIcon))

(event Collision|EventActorBeginOverlap
  (params (OtherActor :type Actor%20Object%20Reference)))

(event EventTick
  (params (DeltaSeconds :type Float%20%28single-precision%29))
  (CallFunction|UpdatePlayerLocation))

(event EventUpdateIcon
  (params (Owner :type Actor%20Object%20Reference) (Data :type F%20Icon%20Data%20Structure))
  (if (CallFunction|FindIcon Owner)
    (CallFunction|UpdateIconData Data Owner))
  (CallFunction|DrawMap)
  (CallFunction|DrawIcon))

(event EventRemoveIcon
  (params (Owner :type Actor%20Object%20Reference))
  (if (CallFunction|FindIcon Owner)
    (CallFunction|RemoveIconData Owner))
  (CallFunction|DrawMap)
  (CallFunction|DrawIcon))

(event EventCreateIcon
  (params (Owner :type Actor%20Object%20Reference) (Data :type F%20Icon%20Data%20Structure))
  (if (not (CallFunction|FindIcon Owner))
    (CallFunction|AddIconData Data Owner)
    (CallFunction|DrawMap)
    (CallFunction|DrawIcon)
    (if (Utilities|Struct|BreakF_IconData Data)
      (Default|CreateIconIndicator (Variables|Default|GetUMG_Minimap) Owner Data 0.0))))

(fn ConstructionScript)

(fn DrawIcon
  (bind _values (Utilities|Map|Values (Variables|Default|GetIconData)))
  (for _array_element _values
    (LocalVariables|SetCurIconData _array_element)
    (Utilities|FlowControl|Sequence
      (:then_0
        (bind _returnvalue (Rendering|Material|GetVectorParameterValue "/Game/MiniMap/Materials/MP_Minimap.MP_Minimap" "MapSize" :!class /Script/Engine.KismetMaterialLibrary))
        (LocalVariables|SetIconUV (Math|Vector2D|MakeVector2D (.y (/ (Utilities|Struct|BreakF_IconData (LocalVariables|GetCurIconData)) (Math|Vector2D|MakeVector2D (.R (Math|Color|BreakColor _returnvalue)) (.G (Math|Color|BreakColor _returnvalue))))) (- 1.0 (.x (/ (Utilities|Struct|BreakF_IconData (LocalVariables|GetCurIconData)) (Math|Vector2D|MakeVector2D (.R (Math|Color|BreakColor _returnvalue)) (.G (Math|Color|BreakColor _returnvalue))))))))
        (goto _label Reset))
      (:then_1
        (Utilities|FlowControl|DoOnce true :!label _label
          (:Completed
            (bind (_canvas _size _context) (Rendering|BeginDrawCanvastoRenderTarget (Variables|Default|GetRT_Map)))
            (Canvas|DrawTexture :self _canvas :RenderTexture (.IconImage (Utilities|Struct|BreakF_IconData (LocalVariables|GetCurIconData))) :ScreenPosition (- (* _size (LocalVariables|GetIconUV)) (* (.Size (Utilities|Struct|BreakF_IconData (LocalVariables|GetCurIconData))) "(X=0.500000,Y=0.500000)")) :ScreenSize (.Size (Utilities|Struct|BreakF_IconData (LocalVariables|GetCurIconData))) :CoordinateSize "(X=1.000000,Y=1.000000)" :PivotPoint "(X=0.500000,Y=0.500000)")
            (Rendering|EndDrawCanvastoRenderTarget _context)))))))

(fn FindIcon
  (params (IconOwner :type Actor%20Object%20Reference))
  (return (.ReturnValue (Utilities|Map|Find (Variables|Default|GetIconData) (Utilities|GetDisplayName IconOwner)))))

(fn DrawMap
  (Rendering|ClearRenderTarget2D (Variables|Default|GetRT_Map))
  (bind (_canvas _size _context) (Rendering|BeginDrawCanvastoRenderTarget (Variables|Default|GetRT_Map)))
  (Canvas|DrawTexture :self _canvas :RenderTexture (Variables|Default|GetCurMapTexture) :ScreenSize _size :CoordinateSize "(X=1.000000,Y=1.000000)" :PivotPoint "(X=0.500000,Y=0.500000)")
  (Rendering|EndDrawCanvastoRenderTarget _context))

(fn AddIconData
  (params (F_IconData :type F%20Icon%20Data%20Structure%20%28by%20ref%29) (IconOwner :type Actor%20Object%20Reference%20%28by%20ref%29))
  (Utilities|Map|Add (Variables|Default|GetIconData) (Utilities|GetDisplayName IconOwner) F_IconData))

(fn RemoveIconData
  (params (IconOwner :type Actor%20Object%20Reference%20%28by%20ref%29))
  (Utilities|Map|Remove (Variables|Default|GetIconData) (Utilities|GetDisplayName IconOwner)))

(fn UpdateIconData
  (params (NewIconData :type F%20Icon%20Data%20Structure%20%28by%20ref%29) (IconOwner :type Actor%20Object%20Reference%20%28by%20ref%29))
  (bind _returnvalue (Utilities|GetDisplayName IconOwner))
  (bind _icondata (Variables|Default|GetIconData))
  (Utilities|Map|Remove _icondata _returnvalue)
  (Utilities|Map|Add _icondata _returnvalue NewIconData))

(fn UpdatePlayerLocation
  (Rendering|Material|SetVectorParameterValue "/Game/MiniMap/Materials/MP_Minimap.MP_Minimap" "PlayerLocation" (Math|Conversions|ToLinearColor(Vector) (Transformation|GetActorLocation (Game|GetPlayerCharacter 0))) :!class /Script/Engine.KismetMaterialLibrary))